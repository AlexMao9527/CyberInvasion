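; Shooter player character that adds an intro sound, an overhead-style name widget and walk speed control.
; BeginPlay plays the sound at the character's location and copies the PlayerState name into the UBP_PlayerName widget.
; OnChangePlayerNameWidget refreshes that name from MPlayerState after a fixed delay, finding the widget component by class.
; OnSetMaxWalkSpeed writes the supplied speed to CharacterMovement.
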(event EventBeginPlay
  (bind _self self)
  (bind _playerstate (Variables|Default|GetPlayerState _self))
  (Audio|PlaySoundatLocation "/Game/AssetPacks/GameDevTV/VoiceOvers/Intro.Intro" (Transformation|GetActorLocation) "0, 0, 0" 1.0 1.0 0.0 0 0 0 0)
  (bind _asubp_player_name (Utilities|Casting|CastToUBP_PlayerName (UserInterface|GetWidget (Variables|Default|GetPlayerNameWidgetComponent))))
  (Utilities|IsValid _playerstate
    (:Is%20Valid
      (Variables|/Game/Buleprint/NormalBuleprint/UBP_PlayerName.UBP_PlayerName_C|SetplayerName _asubp_player_name (PlayerState|GetPlayerName _playerstate)))))

(event Collision|EventActorBeginOverlap
  (params (OtherActor :type Actor%20Object%20Reference)))

(event EventOnSetMaxWalkSpeed
  (params (fNewMaxWaldSpeed :type Float%20%28single-precision%29))
  (Variables|/Script/Engine.CharacterMovementComponent|SetMaxWalkSpeed (Variables|Character|GetCharacterMovement) fNewMaxWaldSpeed))

(event EventOnChangePlayerNameWidget
  (bind _self self)
  (bind _playerstate (Variables|Default|GetPlayerState _self))
  (Utilities|Casting|CastToMPlayerState (Variables|Default|GetPlayerState self))
  (Utilities|FlowControl|Delay 3.0)
  (bind _asubp_player_name (Utilities|Casting|CastToUBP_PlayerName (UserInterface|GetWidget (Actor|GetComponentbyClass "/Script/UMG.WidgetComponent"))))
  (Utilities|IsValid _playerstate
    (:Is%20Valid
      (bind _asmplayer_state (Utilities|Casting|CastToMPlayerState _playerstate))
      (Variables|/Game/Buleprint/NormalBuleprint/UBP_PlayerName.UBP_PlayerName_C|SetplayerName _asubp_player_name (PlayerState|GetPlayerName _asmplayer_state)))))

(fn ConstructionScript)