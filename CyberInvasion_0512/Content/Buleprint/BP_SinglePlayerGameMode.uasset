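; Single-player game mode that handles the lose condition and bot spawning.
; On BeginPlay it binds to actor-killed events and triggers a failed game over when the victim casts to BP_ShooterCharacter.
; SpawnNewBot runs an EQS spawn-location query picking from the best 5% of results.
; On query success, it randomly spawns an AI shooter (less often) or a tracker bot at each returned location.
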(event Custom|OnQueryFinished
  (params (QueryInstance :type Env%20Query%20Instance%20Blueprint%20Wrapper%20Object%20Reference) (QueryStatus :type EEnvQueryStatus%20Enum :default "Processing"))
  (switch Utilities|FlowControl|Switch|SwitchonEEnvQueryStatus QueryStatus
    (:Success
      (bind _resultlocations (AI|EQS|GetQueryResultsasLocations QueryInstance))
      (for _array_element _resultlocations
        (if (<= (Math|Random|RandomFloatinRange 0.0 1e+02) 4e+01)
          (Game|SpawnActorfromClass "/Game/Buleprint/AdvancedAII/BP_AIShooterCharacter.BP_AIShooterCharacter_C" (Math|Transform|MakeTransform _array_element) "AdjustIfPossibleButDontSpawnIfColliding" 0 0)
          (else
            (Game|SpawnActorfromClass "/Game/Buleprint/AdvancedAII/AITrackerBot/BP_TrackerBot.BP_TrackerBot_C" (Math|Transform|MakeTransform _array_element) "AdjustIfPossibleButDontSpawnIfColliding" 0 0)))))))

(event Custom|OnActorKilled_Custom
  (params (victimActor :type Actor%20Object%20Reference) (killerActor :type Actor%20Object%20Reference) (killerController :type Controller%20Object%20Reference))
  (Utilities|Casting|CastToBP_ShooterCharacter victimActor)
  (Class|MSinglePlayerGameMode|GameOverCustom self false))

(event EventBeginPlay
  (EventDispatchers|BindEventtoOnActorKilled (delegate Custom|OnActorKilled_Custom)))

(event EventTick
  (params (DeltaSeconds :type Float%20%28single-precision%29)))

(event EventSpawnNewBot
  (bind _returnvalue (AI|EQS|RunEQSQuery "/Game/Buleprint/AdvancedAII/NormalAIRelated/EQS_FindSpawnLocation.EQS_FindSpawnLocation" self "RandomBest5Pct"))
  (EventDispatchers|BindEventtoOnQueryFinishedEvent _returnvalue (delegate Custom|OnQueryFinished)))

(fn ConstructionScript)