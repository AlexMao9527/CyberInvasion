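; Multiplayer game mode Blueprint that awards kill score and spawns AI bots.
; A kill handler adds points to the killer's MPlayerState, with the amount set by victim type: AI shooter, tracker bot or shooter character.
; SpawnNewBot runs the EQS_FindSpawnLocation query, then on success randomly spawns an AI shooter (favored) or tracker bot at each returned location, adjusting for collisions.
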(event Custom|OnQueryFinished
  (params (QueryInstance :type Env%20Query%20Instance%20Blueprint%20Wrapper%20Object%20Reference) (QueryStatus :type EEnvQueryStatus%20Enum :default "Processing"))
  (switch Utilities|FlowControl|Switch|SwitchonEEnvQueryStatus QueryStatus
    (:Success
      (bind _resultlocations (AI|EQS|GetQueryResultsasLocations QueryInstance))
      (for _array_element _resultlocations
        (if (<= (Math|Random|RandomFloatinRange 0.0 1e+02) 6e+01)
          (Game|SpawnActorfromClass "/Game/Buleprint/AdvancedAII/BP_AIShooterCharacter.BP_AIShooterCharacter_C" (Math|Transform|MakeTransform _array_element) "AdjustIfPossibleButDontSpawnIfColliding" 0 0)
          (else
            (Game|SpawnActorfromClass "/Game/Buleprint/AdvancedAII/AITrackerBot/BP_TrackerBot.BP_TrackerBot_C" (Math|Transform|MakeTransform _array_element) "AdjustIfPossibleButDontSpawnIfColliding" 0 0)))))))

(event Custom|CustomEvent_0
  (params (victimActor :type Actor%20Object%20Reference) (killerActor :type Actor%20Object%20Reference) (killerController :type Controller%20Object%20Reference))
  (bind _playerstate (Variables|/Script/Engine.Controller|GetPlayerState killerController))
  (Utilities|IsValid killerController
    (:Is%20Valid
      (Utilities|Casting|CastToMAIShooterCharacter victimActor
        (:then
          (Utilities|IsValid _playerstate
            (:Is%20Valid
              (bind _asmplayer_state (Utilities|Casting|CastToMPlayerState _playerstate))
              (Utilities|IsValid _asmplayer_state
                (:Is%20Valid
                  (Class|MPlayerState|AddScore _asmplayer_state 3e+01))))))
        (:CastFailed
          (Utilities|Casting|CastToMTrackerBot victimActor
            (:then
              (Utilities|IsValid _playerstate
                (:Is%20Valid
                  (bind _asmplayer_state_2 (Utilities|Casting|CastToMPlayerState _playerstate))
                  (Utilities|IsValid _asmplayer_state_2
                    (:Is%20Valid
                      (Class|MPlayerState|AddScore _asmplayer_state_2 5.0))))))
            (:CastFailed
              (Utilities|Casting|CastToMShooterCharacter victimActor)
              (Utilities|IsValid _playerstate
                (:Is%20Valid
                  (bind _asmplayer_state_3 (Utilities|Casting|CastToMPlayerState _playerstate))
                  (Utilities|IsValid _asmplayer_state_3
                    (:Is%20Valid
                      (Class|MPlayerState|AddScore _asmplayer_state_3 5e+01))))))))))))

(event EventBeginPlay
  (EventDispatchers|BindEventtoOnActorKilled (delegate Custom|CustomEvent_0)))

(event EventTick
  (params (DeltaSeconds :type Float%20%28single-precision%29)))

(event EventSpawnNewBot
  (bind _returnvalue (AI|EQS|RunEQSQuery "/Game/Buleprint/AdvancedAII/NormalAIRelated/EQS_FindSpawnLocation.EQS_FindSpawnLocation" self "RandomBest5Pct"))
  (EventDispatchers|BindEventtoOnQueryFinishedEvent _returnvalue (delegate Custom|OnQueryFinished)))

(fn ConstructionScript)