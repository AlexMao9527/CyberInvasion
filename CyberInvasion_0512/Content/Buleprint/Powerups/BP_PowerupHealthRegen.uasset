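; BP_PowerupHealthRegen is a powerup actor that heals the character that activates it over successive powerup ticks.
; OnActivated stores the activating actor, and each OnPowerupTicked casts it to MShooterCharacter and calls Heal on its HealthComponent with HealAmountPerTick.
; OnPowerupStateChanged always hides the mesh and point light, propagating to their children, without reading the new state.
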(event EventBeginPlay)

(event Collision|EventActorBeginOverlap
  (params (OtherActor :type Actor%20Object%20Reference)))

(event EventTick
  (params (DeltaSeconds :type Float%20%28single-precision%29)))

(event EventOnActivated
  (params (activeFor :type Actor%20Object%20Reference))
  (Variables|Default|SetActiveFor activeFor))

(event EventOnPowerupTicked
  (bind _activefor (Variables|Default|GetActiveFor))
  (Utilities|IsValid _activefor
    (:Is%20Valid
      (bind _asmshooter_character (Utilities|Casting|CastToMShooterCharacter _activefor))
      (Utilities|IsValid _asmshooter_character
        (:Is%20Valid
          (Class|MHealthComponent|Heal (Variables|/Script/CyberInvasion.MShooterCharacter|GethealthComponent _asmshooter_character) (Variables|Default|GethealAmountPerTick)))))))

(event EventOnPowerupStateChanged
  (params (bNewIsPowerupActive :type Boolean))
  (Rendering|SetVisibility (Variables|Default|GetmeshComp) false true)
  (Rendering|SetVisibility (Variables|Default|GetPointLight) false true))

(fn ConstructionScript)