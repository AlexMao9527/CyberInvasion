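; Super speed powerup that temporarily doubles the walk speed of the actor it activates for.
; On activation it stores that actor and doubles its CharacterMovementComponent MaxWalkSpeed; on expiry it halves the current value to undo the boost.
; Both events copy the new speed into CurMaxWalkSpeed when the actor is an MShooterCharacter.
; A powerup state change hides the mesh and its children.
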(event EventBeginPlay)

(event Collision|EventActorBeginOverlap
  (params (OtherActor :type Actor%20Object%20Reference)))

(event EventOnActivated
  (params (activeFor :type Actor%20Object%20Reference))
  (Variables|Default|SetActiveFor activeFor)
  (Variables|/Script/Engine.CharacterMovementComponent|SetMaxWalkSpeed (Actor|GetComponentbyClass (Variables|Default|GetActiveFor) "/Script/Engine.CharacterMovementComponent") (* (Variables|/Script/Engine.CharacterMovementComponent|GetMaxWalkSpeed (Actor|GetComponentbyClass (Variables|Default|GetActiveFor) "/Script/Engine.CharacterMovementComponent")) 2.0))
  (bind _asmshooter_character (Utilities|Casting|CastToMShooterCharacter (Variables|Default|GetActiveFor)))
  (Variables|/Script/CyberInvasion.MShooterCharacter|SetcurMaxWalkSpeed _asmshooter_character (Variables|/Script/Engine.CharacterMovementComponent|GetMaxWalkSpeed (Actor|GetComponentbyClass (Variables|Default|GetActiveFor) "/Script/Engine.CharacterMovementComponent"))))

(event EventOnExpired
  (bind _activefor (Variables|Default|GetActiveFor))
  (bind _returnvalue (Actor|GetComponentbyClass _activefor "/Script/Engine.CharacterMovementComponent"))
  (Variables|/Script/Engine.CharacterMovementComponent|SetMaxWalkSpeed _returnvalue (/ (Variables|/Script/Engine.CharacterMovementComponent|GetMaxWalkSpeed _returnvalue) 2.0))
  (bind _asmshooter_character (Utilities|Casting|CastToMShooterCharacter _activefor))
  (Variables|/Script/CyberInvasion.MShooterCharacter|SetcurMaxWalkSpeed _asmshooter_character (Variables|/Script/Engine.CharacterMovementComponent|GetMaxWalkSpeed _returnvalue)))

(event EventOnPowerupStateChanged
  (params (bNewIsPowerupActive :type Boolean))
  (Rendering|SetVisibility (Variables|Default|GetmeshComp) false true))

(fn ConstructionScript)